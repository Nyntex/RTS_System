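; In-game Game Mode that assigns each player a spawn point and prints their PlayerId on login.
; ChoosePlayerStart looks up the PlayerId in BP_GameInstance's PlayerSpawnpoints map and returns the PlayerStart with the matching tag.
; Players missing from the map get the first PlayerStart found.
; The logout actor search takes no action, and a delayed StartMatch and a "Taken"-tag spawn method are left unconnected.
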(event `self.ReceiveBeginPlay`)

(event `self.K2_PostLogin`
  (params (NewPlayer :type "PlayerController Object Reference"))
  (`KismetSystemLibrary.PrintString` (`KismetStringLibrary.Conv_IntToString` (`PlayerState.PlayerId` (`Controller.PlayerState` NewPlayer))) true true (struct :`R` 1.0 :`B` 0.787428 :`A` 1.0) 10.0))

(event `self.K2_OnLogout`
  (params (ExitingController :type "Controller Object Reference"))
  (bind _outactors (`GameplayStatics.GetAllActorsOfClass` "/Script/Engine.Actor"))
  (for _array_element _outactors
    (bind _asbp_player_character (cast `/Game/Player/BP_PlayerCharacter` (`self.GetOwner` _array_element)))
    (if (== (`Controller.PlayerState` (`Pawn.GetController` _asbp_player_character)) (`Controller.PlayerState` ExitingController))
      _)))

(fn `ChoosePlayerStart`
  (params (Player :type "Controller Object Reference"))
  (returns (ReturnValue :type "Actor Object Reference"))
  (bind _asbp_player_state (cast `/Game/Player/BP_PlayerState` (`Controller.PlayerState` Player)))
  (bind _asbp_game_instance (cast `/Game/GeneralLogic/BP_GameInstance` (`GameplayStatics.GetGameInstance`)))
  (bind _playerspawnpoints (`/Game/GeneralLogic/BP_GameInstance.PlayerSpawnpoints` _asbp_game_instance))
  (bind _keys (`BlueprintMapLibrary.Map_Keys` _playerspawnpoints))
  (bind _values (`BlueprintMapLibrary.Map_Values` _playerspawnpoints))
  (bind _returnvalue (`KismetArrayLibrary.Array_Find` _keys (`PlayerState.PlayerId` _asbp_player_state)))
  (if (== _returnvalue -1)
    (bind _outactors (`GameplayStatics.GetAllActorsOfClass` "/Script/Engine.PlayerStart"))
    (return (`|GetArrayItem` _outactors))
    (else
      (bind _outactors_2 (`GameplayStatics.GetAllActorsOfClass` "/Script/Engine.PlayerStart"))
      (for _array_element _outactors_2
        (if (== (`PlayerStart.PlayerStartTag` _array_element) (`KismetStringLibrary.Conv_StringToName` (`KismetStringLibrary.Conv_IntToString` (`|GetArrayItem` _values _returnvalue))))
          (`|ExecutionSequence`
            (:`then_0`
              (`KismetSystemLibrary.PrintString` "found spawnpoint")
              (return _array_element))
            (:`then_1`
              (break))))))))

(fn `UserConstructionScript`)