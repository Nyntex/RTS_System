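; BP_BaseBuilding is the base faction building actor, handling hover and selection feedback plus a construction-complete check.
; Hover and selection events toggle gameplay tags, which drive the mesh's custom depth rendering for highlighting.
; On BeginPlay, the stencil value is set by whether the local player's ID matches the owning PlayerState's, distinguishing own buildings from others.
; Selecting also shows a widget on the player screen, removed on deselect.
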(event `self.ReceiveBeginPlay`
  (`self.SetHoverMaterialDepthNumberByRelation` (`Controller.PlayerState` (`GameplayStatics.GetPlayerController` 0))))

(event `/Game/GeneralLogic/Interfaces/BPI_Selectable.Hover`
  (`BlueprintGameplayTagLibrary.AddGameplayTag` (`self.GameplayTags`) (struct :`TagName` "Selection.Hovering"))
  (`self.SetRenderCustomDepthBySelection`))

(event `/Game/GeneralLogic/Interfaces/BPI_Selectable.StopHover`
  (`BlueprintGameplayTagLibrary.RemoveGameplayTag` (`self.GameplayTags`) (struct :`TagName` "Selection.Hovering"))
  (`self.SetRenderCustomDepthBySelection`))

(event `/Game/GeneralLogic/Interfaces/BPI_Selectable.Select`
  (bind _returnvalue (`|CreateWidget` (`self.SelectedWidget`) (`GameplayStatics.GetPlayerController` 0)))
  (bind _output_get (set `self.ActiveWidget` _returnvalue))
  (`UserWidget.AddToPlayerScreen` _output_get 0)
  (`BlueprintGameplayTagLibrary.AddGameplayTag` (`self.GameplayTags`) (struct :`TagName` "Selection.Selected"))
  (`self.SetRenderCustomDepthBySelection`))

(event `/Game/GeneralLogic/Interfaces/BPI_Selectable.Deselect`
  (`Widget.RemoveFromParent` (`self.ActiveWidget`))
  (set `self.ActiveWidget` null)
  (`BlueprintGameplayTagLibrary.RemoveGameplayTag` (`self.GameplayTags`) (struct :`TagName` "Selection.Selected"))
  (`self.SetRenderCustomDepthBySelection`))

(fn `FinishedConstruction`
  (returns (ReturnValue :type Boolean))
  (return (>= (`self.ConstructionProgress`) 100.0)))

(fn `GetOwningPlayerState`
  (returns (`Player State` :type "PlayerState Object Reference"))
  (bind _asplayer_state (cast `PlayerState` (`self.GetOwner`))
    (:`then`
      (return _asplayer_state))
    (:`CastFailed`
      (return null))))

(fn `SetHoverMaterialDepthNumberByRelation`
  (params (PlayerToCheck :type "PlayerState Object Reference"))
  (bind _mesh (`self.Mesh`))
  (if (== (`PlayerState.PlayerId` PlayerToCheck) (`PlayerState.PlayerId` (`self.GetOwningPlayerState`)))
    (`PrimitiveComponent.SetCustomDepthStencilValue` _mesh 1)
    (else
      (`PrimitiveComponent.SetCustomDepthStencilValue` _mesh 3))))

(fn `SetRenderCustomDepthBySelection`
  (`PrimitiveComponent.SetRenderCustomDepth` (`self.Mesh`) (or (`BlueprintGameplayTagLibrary.HasTag` (`self.GameplayTags`) (struct :`TagName` "Selection.Hovering")) (`BlueprintGameplayTagLibrary.HasTag` (`self.GameplayTags`) (struct :`TagName` "Selection.Selected"))))
  (return))

(fn `UserConstructionScript`)