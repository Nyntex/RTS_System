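; BP_BaseBuilding is a building actor that highlights on hover according to whether the local player owns it.
; On BeginPlay it compares player 0's PlayerId with that of its owner, cast to PlayerState, and picks an own or other stencil value.
; Hover events write that value to the mesh's custom depth stencil and clear it when hovering stops.
; A helper reports whether construction progress has reached completion.
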(event `self.ReceiveBeginPlay`
  (`self.SetHoverMaterialDepthNumberByRelation` (`Controller.PlayerState` (`GameplayStatics.GetPlayerController` 0))))

(event `/Game/GeneralLogic/Interfaces/BPI_Selectable.Hover`
  (`PrimitiveComponent.SetCustomDepthStencilValue` (`self.Mesh`) (`self.HoverMaterialDepthNumber`)))

(event `/Game/GeneralLogic/Interfaces/BPI_Selectable.StopHover`
  (`PrimitiveComponent.SetCustomDepthStencilValue` (`self.Mesh`) 0))

(fn `FinishedConstruction`
  (returns (ReturnValue :type Boolean))
  (return (>= (`self.ConstructionProgress`) 100.0)))

(fn `GetOwningPlayerState`
  (returns (`Player State` :type "PlayerState Object Reference"))
  (bind _asplayer_state (cast `PlayerState` (`self.GetOwner`))
    (:`then`
      (return _asplayer_state))
    (:`CastFailed`
      (return null))))

(fn `SetHoverMaterialDepthNumberByRelation`
  (params (PlayerToCheck :type "PlayerState Object Reference"))
  (if (== (`PlayerState.PlayerId` PlayerToCheck) (`PlayerState.PlayerId` (`self.GetOwningPlayerState`)))
    (set `self.HoverMaterialDepthNumber` 1)
    (else
      (set `self.HoverMaterialDepthNumber` 3))))

(fn `UserConstructionScript`)