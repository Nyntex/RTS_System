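; Blueprint function library of global helpers, holding one function that converts a world position into a building position.
; ConvertPositionToBuildingPosition snaps X and Y to a 50-unit grid by dividing, truncating and multiplying back, and leaves Z unchanged.
; Truncation rounds toward zero rather than to the nearest cell, so negative and positive coordinates snap in opposite directions.
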(fn `ConvertPositionToBuildingPosition`
  (params (Position :type "Vector Structure"))
  (returns (`Building Position` :type "Vector Structure"))
  (return (`KismetMathLibrary.MakeVector` (`KismetMathLibrary.Conv_IntToDouble` (* (`KismetMathLibrary.FTrunc` (/ (.x Position) 50.0)) 50)) (`KismetMathLibrary.Conv_IntToDouble` (* (`KismetMathLibrary.FTrunc` (/ (.y Position) 50.0)) 50)) (.z Position))))