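; RTS HUD that adds the main HUD widget at BeginPlay and handles drag-box selection.
; Press and hold events track mouse corners, starting the marquee only after a drag threshold.
; While dragging, DrawHUD draws a green outline and rebuilds the selection from BPI_Selectable actors inside it, sending hover messages.
; A DoOnce clears hover states when dragging ends, leaving the selection retrievable through a getter.
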(event `self.ReceiveBeginPlay`
  (bind _returnvalue (`|CreateWidget` (`self.MainHudWidget`) (`GameplayStatics.GetPlayerController` 0)))
  (bind _output_get (set `self.HudWidget` _returnvalue))
  (`UserWidget.AddToPlayerScreen` _output_get 0))

(event `/Game/Blueprints/Interfaces/BPI_SelectionMarquee.MarqueePressed`
  (bind (_locationx _locationy) (`PlayerController.GetMousePosition` (`GameplayStatics.GetPlayerController` 0)))
  (bind _output_get (set `self.PointA` (`KismetMathLibrary.MakeVector2D` _locationx _locationy)))
  (set `self.PointB` _output_get)
  (`KismetArrayLibrary.Array_Clear` (`self.CurrentSelection`)))

(event `/Game/Blueprints/Interfaces/BPI_SelectionMarquee.MarqueeHeld`
  (bind (_locationx _locationy) (`PlayerController.GetMousePosition` (`GameplayStatics.GetPlayerController` 0)))
  (bind (_locationx_2 _locationy_2) (`PlayerController.GetMousePosition` (`GameplayStatics.GetPlayerController` 0)))
  (if (`self.DrawingMarquee`)
    (set `self.PointB` (`KismetMathLibrary.MakeVector2D` _locationx_2 _locationy_2))
    (elif (>= (`KismetMathLibrary.Distance2D` (`self.PointA`) (`KismetMathLibrary.MakeVector2D` _locationx _locationy)) (`self.DrawMarqueeThreshold`))
      (set `self.DrawingMarquee` true))))

(event `self.ReceiveDrawHUD`
  (params (SizeX :type Integer) (SizeY :type Integer))
  (if (`self.DrawingMarquee`)
    (`|ExecutionSequence`
      (:`then_0`
        (`self.DrawMarquee`)
        (`self.HoverMarquee`))
      (:`then_1`
        (goto _label :!via `Reset`)))
    (else
      (`/Engine/EditorBlueprintResources/StandardMacros.DoOnce` false :!label _label
        (:`Completed`
          (for _array_element (`self.CurrentSelection`)
            (message `/Game/Blueprints/Interfaces/BPI_Selectable.StopHover` _array_element)))))))

(fn `DrawMarquee`
  (locals (LocalThickness :type "Float (double-precision)" :default 2.0))
  (bind _pointa_x (`KismetMathLibrary.BreakVector2D` (`self.PointA`)))
  (bind (_pointb_x _pointb_y) (`KismetMathLibrary.BreakVector2D` (`self.PointB`)))
  (bind (_pointb_x_2 _pointb_y_2) (`KismetMathLibrary.BreakVector2D` (`self.PointB`)))
  (bind _localthickness (`local.LocalThickness`))
  (bind (_pointa_x_2 _pointa_y) (`KismetMathLibrary.BreakVector2D` (`self.PointA`)))
  (bind _pointb_x_3 (`KismetMathLibrary.BreakVector2D` (`self.PointB`)))
  (bind (_pointa_x_3 _pointa_y_2) (`KismetMathLibrary.BreakVector2D` (`self.PointA`)))
  (bind (_pointb_x_4 _pointb_y_3) (`KismetMathLibrary.BreakVector2D` (`self.PointB`)))
  (bind (_pointa_x_4 _pointa_y_3) (`KismetMathLibrary.BreakVector2D` (`self.PointA`)))
  (`self.DrawRect` (struct :`G` 1.0 :`A` 1.0) _pointa_x_2 _pointa_y (- _pointb_x_3 _pointa_x_2) (`local.LocalThickness`))
  (`self.DrawRect` (struct :`G` 1.0 :`A` 1.0) _pointa_x_3 _pointa_y_2 (`local.LocalThickness`) (- _pointb_y_3 _pointa_y_2))
  (`self.DrawRect` (struct :`G` 1.0 :`A` 1.0) _pointa_x _pointb_y (- _pointb_x _pointa_x) (`local.LocalThickness`))
  (`self.DrawRect` (struct :`G` 1.0 :`A` 1.0) _pointb_x_2 _pointa_y_3 _localthickness (+ (- _pointb_y_2 _pointa_y_3) _localthickness)))

(fn `HoverMarquee`
  (for _array_element (`self.CurrentSelection`)
    (message `/Game/Blueprints/Interfaces/BPI_Selectable.StopHover` _array_element))
  (`KismetArrayLibrary.Array_Clear` (`self.CurrentSelection`))
  (for _array_element_2 (`self.GetActorsInSelectionRectangle` "/Script/Engine.Actor" (`self.PointA`) (`self.PointB`))
    (if (`KismetSystemLibrary.DoesImplementInterface` _array_element_2 "/Game/Blueprints/Interfaces/BPI_Selectable.BPI_Selectable_C")
      (message `/Game/Blueprints/Interfaces/BPI_Selectable.Hover` _array_element_2)
      (`KismetArrayLibrary.Array_AddUnique` (`self.CurrentSelection`) _array_element_2))))

(fn `IsDrawingMarquee`
  (returns (Drawing :type Boolean))
  (return (`self.DrawingMarquee`)))

(fn `MarqueeReleased`
  (set `self.DrawingMarquee` false)
  (return))

(fn `ReceiveMarqueeSelection`
  (returns (SelectedActors :type "Array of Actor Object Reference"))
  (return (`self.CurrentSelection`)))

(fn `UserConstructionScript`)