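; Main menu game mode that clears leftover session data and hands out unique player starts.
; On BeginPlay, TryClearSessionData calls DestroySession for the first player controller and calls Clear on BP_GameInstance from that node's Then output.
; The ChoosePlayerStart override picks the first PlayerStart not tagged "Taken" and tags it so later players get a different one.
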(event `self.ReceiveBeginPlay`
  (`DestroySessionCallbackProxy.DestroySession` (`GameplayStatics.GetPlayerController` 0)
    (:`then`
      (bind _asbp_game_instance (cast `/Game/Blueprints/GeneralLogic/BP_GameInstance` (`GameplayStatics.GetGameInstance`)))
      (`/Game/Blueprints/GeneralLogic/BP_GameInstance.Clear` _asbp_game_instance))))

(fn `ChoosePlayerStart`
  (params (Player :type "Controller Object Reference"))
  (returns (ReturnValue :type "Actor Object Reference"))
  (bind _outactors (`GameplayStatics.GetAllActorsOfClass` "/Script/Engine.PlayerStart"))
  (for _array_element _outactors
    (if (!= (`PlayerStart.PlayerStartTag` _array_element) "Taken")
      (`|ExecutionSequence`
        (:`then_0`
          (break))
        (:`then_1`
          (set `PlayerStart.PlayerStartTag` "Taken" _array_element)
          (return _array_element))))))

(fn `UserConstructionScript`)