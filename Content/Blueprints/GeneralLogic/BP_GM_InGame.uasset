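; In-game game mode that gives each player a start point and a main building.
; It matches the spawn point stored in the game instance's PlayerInfos to a tagged PlayerStart, falling back to the first one for unknown players.
; A tick after player setup, it spawns a building owned by the PlayerState, positioned by grid conversion and downward trace.
; Logout gathers the player's buildings and units but leaves them untouched; debug prints and drawing remain.
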(event `self.ReceiveBeginPlay`)

(event `self.K2_PostLogin`
  (params (NewPlayer :type "PlayerController Object Reference"))
  (`KismetSystemLibrary.PrintString` (`KismetStringLibrary.Concat_StrStr` (`KismetStringLibrary.Conv_IntToString` (`PlayerState.PlayerId` (`Controller.PlayerState` NewPlayer))) " login") true true (struct :`R` 1.0 :`B` 0.787428 :`A` 1.0) 10.0))

(event `self.K2_OnLogout`
  (params (ExitingController :type "Controller Object Reference"))
  (`self.GetActorsOfPlayer` (`Controller.PlayerState` ExitingController)))

(event `self.HandleStartingNewPlayer`
  (params (NewPlayer :type "PlayerController Object Reference"))
  (`parent.HandleStartingNewPlayer` NewPlayer)
  (`KismetSystemLibrary.DelayUntilNextTick`)
  (bind _asbp_player_state (cast `/Game/Blueprints/Player/BP_PlayerState` (`Controller.PlayerState` NewPlayer)))
  (bind _spawnpoint (`self.GetSpawnPointForPlayer` NewPlayer))
  (bind _buildingspawnposition (`self.Get Main Building Spawn Position` (`self.K2_GetActorLocation` _spawnpoint)))
  (`KismetSystemLibrary.PrintString` (`KismetStringLibrary.Conv_VectorToString` _buildingspawnposition) true true (struct :`G` 0.66 :`B` 1.0 :`A` 1.0) 100.0)
  (`|SpawnActorFromClass` "/Game/Blueprints/Factions/Base/BP_BaseBuilding.BP_BaseBuilding_C" (`KismetMathLibrary.MakeTransform` _buildingspawnposition) "Undefined" "MultiplyWithRoot" _asbp_player_state _asbp_player_state null))

(fn `ChoosePlayerStart`
  (params (Player :type "Controller Object Reference"))
  (returns (ReturnValue :type "Actor Object Reference"))
  (bind _spawnpoint (`self.GetSpawnPointForPlayer` Player))
  (return _spawnpoint))

(fn `Get Main Building Spawn Position`
  (params (PlayerSpawnPosition :type "Vector Structure"))
  (returns (BuildingSpawnPosition :type "Vector Structure"))
  (bind _returnvalue (`UtilityFunctions.ConvertPositionToBuildingPosition` PlayerSpawnPosition 250.0))
  (bind _outhit (`KismetSystemLibrary.LineTraceSingle` :`Start` _returnvalue :`End` (+ _returnvalue (* (`KismetMathLibrary.Vector_Down`) 10000.0)) :`TraceChannel` "TraceTypeQuery1" :`DrawDebugType` "ForDuration" :`bIgnoreSelf` false))
  (bind (_bblockinghit _binitialoverlap _time _distance _location) (`GameplayStatics.BreakHitResult` _outhit))
  (`KismetSystemLibrary.DrawDebugSphere` _location 100.0 12 (struct :`R` 1.0 :`G` 1.0 :`B` 1.0 :`A` 1.0) 10.0 20.0)
  (return _location))

(fn `GetActorsOfPlayer`
  (params (PlayerState :type "PlayerState Object Reference"))
  (returns (ActorsOfPlayerState :type "Array of Actor Object Reference"))
  (locals (PossibleActors :type "Array of Actor Object Reference") (OwnedActors :type "Array of Actor Object Reference"))
  (bind _possibleactors (`local.PossibleActors`))
  (`KismetArrayLibrary.Array_Clear` _possibleactors)
  (bind _outactors (`GameplayStatics.GetAllActorsOfClass` "/Game/Blueprints/Factions/Base/BP_BaseBuilding.BP_BaseBuilding_C"))
  (`KismetArrayLibrary.Array_Append` _possibleactors _outactors)
  (bind _outactors_2 (`GameplayStatics.GetAllActorsOfClass` "/Game/Blueprints/Factions/Base/BP_BaseUnit.BP_BaseUnit_C"))
  (`KismetArrayLibrary.Array_Append` _possibleactors _outactors_2)
  (for _array_element (`local.PossibleActors`)
    (bind _asbp_player_character (cast `/Game/Blueprints/Player/BP_PlayerCharacter` (`self.GetOwner` _array_element)))
    (bind _returnvalue (`Pawn.GetController` _asbp_player_character))
    (`/Engine/EditorBlueprintResources/StandardMacros.IsValid` _returnvalue
      (:`Is Valid`
        (if (== (`Controller.PlayerState` _returnvalue) (`local.PlayerState`))
          (`KismetArrayLibrary.Array_AddUnique` (`local.OwnedActors`) _array_element)))))
  (return (`local.OwnedActors`)))

(fn `GetSpawnPointForPlayer`
  (params (PlayerController :type "Controller Object Reference"))
  (returns (Spawnpoint :type "PlayerStart Object Reference"))
  (bind _asbp_game_instance (cast `/Game/Blueprints/GeneralLogic/BP_GameInstance` (`GameplayStatics.GetGameInstance`)))
  (bind (_value _returnvalue) (`BlueprintMapLibrary.Map_Find` (`/Game/Blueprints/GeneralLogic/BP_GameInstance.PlayerInfos` _asbp_game_instance) (`PlayerState.PlayerId` (`Controller.PlayerState` PlayerController))))
  (if _returnvalue
    (bind _outactors (`GameplayStatics.GetAllActorsOfClass` "/Script/Engine.PlayerStart"))
    (for _array_element _outactors
      (if (`self.ActorHasTag` _array_element (`KismetStringLibrary.Conv_StringToName` (`KismetStringLibrary.Conv_IntToString` (break `/Game/Blueprints/Structures/STR_PlayerInfo` _value))))
        (return _array_element)))
    (else
      (bind _outactors_2 (`GameplayStatics.GetAllActorsOfClass` "/Script/Engine.PlayerStart"))
      (if (> (`KismetArrayLibrary.Array_Length` _outactors_2) 0)
        (return (`|GetArrayItem` _outactors_2))
        (else
          (return null))))))

(fn `UserConstructionScript`)