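; BP_GameState is the game state that refreshes lobby player lists and resolves spawnpoint conflicts between players.
; UpdatePlayerList and the AllPlayerStates OnRep both call UpdateList on every WBP_LobbyMenu widget.
; ValidateSpawnpoint scans PlayerArray, skipping the ignored state, and advances a clashing spawnpoint index, wrapping from 8 to 1.
; It recurses until the index stays unchanged, with no guard for all slots being taken.
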(event `self.ReceiveBeginPlay`)

(event `UpdatePlayerList`
  (bind _foundwidgets (`WidgetBlueprintLibrary.GetAllWidgetsOfClass` "/Game/Blueprints/Lobby/UI/WBP_LobbyMenu.WBP_LobbyMenu_C" false))
  (for _array_element _foundwidgets
    (`/Game/Blueprints/Lobby/UI/WBP_LobbyMenu.UpdateList` _array_element)))

(fn `OnRep_AllPlayerStates`
  (bind _foundwidgets (`WidgetBlueprintLibrary.GetAllWidgetsOfClass` "/Game/Blueprints/Lobby/UI/WBP_LobbyMenu.WBP_LobbyMenu_C" false))
  (for _array_element _foundwidgets
    (`/Game/Blueprints/Lobby/UI/WBP_LobbyMenu.UpdateList` _array_element)))

(fn `UserConstructionScript`)

(fn `ValidateSpawnpoint`
  (params (ToValidate :type Integer) (StateToIgnore :type "/Game/Blueprints/Player/BP_PlayerState Object Reference"))
  (returns (Validated :type Integer))
  (locals (retVal :type Integer))
  (set `local.retVal` ToValidate)
  (for _array_element (`GameStateBase.PlayerArray` (`GameplayStatics.GetGameState`))
    (bind _asbp_player_state (cast `/Game/Blueprints/Player/BP_PlayerState` _array_element))
    (if (== _asbp_player_state StateToIgnore)
      _
      (elif (== (`/Game/Blueprints/Player/BP_PlayerState.Spawnpoint` _asbp_player_state) (`local.retVal`))
        (if (== (`local.retVal`) 8)
          (set `local.retVal` 1)
          (else
            (`/Engine/EditorBlueprintResources/StandardMacros.IncrementInt` (`local.retVal`)))))))
  (if (== (`local.retVal`) (`local.ToValidate`))
    (return (`local.ToValidate`))
    (else
      (bind _validated (`self.ValidateSpawnpoint` (`local.retVal`) (`local.StateToIgnore`)))
      (return _validated))))