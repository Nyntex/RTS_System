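; Player State Blueprint that holds a player's chosen faction and spawn point.
; A server update event forwards both values to a client update event, which stores them on the player state.
; The client event also writes them, with the player's allies, into the Game Instance's player info map keyed by player ID, then fires a settings-changed notification.
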(event `self.ReceiveBeginPlay`)

(event `UpdateSettings (Server)`
  (params (Faction :type "/Game/Blueprints/Enum/EFactions Enum" :default "NewEnumerator0") (Spawnpoint :type Integer))
  (`self.UpdateSettings (Client)` Faction Spawnpoint))

(event `UpdateSettings (Client)`
  (params (Faction :type "/Game/Blueprints/Enum/EFactions Enum" :default "NewEnumerator0") (Spawnpoint :type Integer))
  (set `self.Faction` Faction)
  (set `self.Spawnpoint` Spawnpoint)
  (bind _asbp_game_instance (cast `/Game/Blueprints/GeneralLogic/BP_GameInstance` (`GameplayStatics.GetGameInstance`)))
  (`BlueprintMapLibrary.Map_Add` (`/Game/Blueprints/GeneralLogic/BP_GameInstance.PlayerInfos` _asbp_game_instance) (`self.PlayerId`) (make `/Game/Blueprints/Structures/STR_PlayerInfo` (`self.Spawnpoint`) (`self.Faction`) (`self.Allies`)))
  (`self.SettingsChanged`))

(fn `UserConstructionScript`)