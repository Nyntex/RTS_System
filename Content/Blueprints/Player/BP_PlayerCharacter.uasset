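; Player pawn for a top-down building game, with a spring-arm camera driven by Enhanced Input.
; Move input offsets the actor without sweep, scroll changes arm length with only a lower limit, and rotation comes from an input axis or mouse drag, with invert options.
; A test key traces from the cursor, converts the hit to a building position and asks the server to spawn a base building owned by the player state.
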(event `self.ReceiveBeginPlay`
  (`self.AddMappingContext`)
  (`self.SetInitialValues`))

(event `self.ReceiveTick`
  (params (DeltaSeconds :type "Float (single-precision)")))

(event `EnhancedInput|/Game/Input/InputActions/Player/IA_Player_EnableCameraRotation`
  (params (ActionValue :type Boolean) (ElapsedSeconds :type "Float (double-precision)") (TriggeredSeconds :type "Float (double-precision)") (InputAction :type "InputAction Object Reference" :default "/Game/Input/InputActions/Player/IA_Player_EnableCameraRotation.IA_Player_EnableCameraRotation"))
  (:`Started`
    (bind _returnvalue (`WidgetLayoutLibrary.GetMousePositionOnViewport`))
    (bind _output_get (set `self.CameraRotationStart` _returnvalue))
    (set `self.CameraRotationOngoing` _output_get))
  (:`Ongoing`
    (bind _returnvalue_2 (`WidgetLayoutLibrary.GetMousePositionOnViewport`))
    (set `self.CameraRotationOngoing` _returnvalue_2)
    (`self.RotateCameraByVector2` (/ (- (`self.CameraRotationOngoing`) (`self.CameraRotationStart`)) 10.0))
    (set `self.CameraRotationStart` (`self.CameraRotationOngoing`))))

(event `Key|Two`
  (params (Key :type "Key Structure"))
  ;[1 0.1557 0.1458] TESTING
  (:`Pressed`
    (bind _location (`self.LineTraceFromMouseToWorld` 10000.0))
    (bind _asbp_player_state (cast `/Game/Blueprints/Player/BP_PlayerState` (`self.PlayerState`)))
    (`self.TrySpawnBuilding (Server)` "/Game/Blueprints/Factions/Base/BP_BaseBuilding.BP_BaseBuilding_C" (`UtilityFunctions.ConvertPositionToBuildingPosition` _location 250.0) _asbp_player_state)))

(event `EnhancedInput|/Game/Input/InputActions/Player/IA_Player_RotateCamera`
  (params (ActionValue :type "Vector2D Structure") (ElapsedSeconds :type "Float (double-precision)") (TriggeredSeconds :type "Float (double-precision)") (InputAction :type "InputAction Object Reference" :default "/Game/Input/InputActions/Player/IA_Player_RotateCamera.IA_Player_RotateCamera"))
  (:`Triggered`
    (`self.RotateCameraByVector2` ActionValue :!label _label))
  (:`Started`
    (goto _label))
  (:`Ongoing`
    (goto _label))
  (:`Completed`
    (goto _label)))

(event `TrySpawnBuilding (Server)`
  (params (Class :type "/Game/Blueprints/Factions/Base/BP_BaseBuilding Class Reference") (`Spawn Transform Location` :type "Vector Structure") (Owner :type "/Game/Blueprints/Player/BP_PlayerState Object Reference"))
  (`|SpawnActorFromClass` Class (`KismetMathLibrary.MakeTransform` `Spawn Transform Location`) "AlwaysSpawn" "MultiplyWithRoot" Owner Owner null))

(event `EnhancedInput|/Game/Input/InputActions/Player/IA_Player_Move`
  (params (ActionValue :type "Vector2D Structure") (ElapsedSeconds :type "Float (double-precision)") (TriggeredSeconds :type "Float (double-precision)") (InputAction :type "InputAction Object Reference" :default "/Game/Input/InputActions/Player/IA_Player_Move.IA_Player_Move"))
  (bind (_x _y) (`KismetMathLibrary.BreakVector2D` ActionValue))
  (:`Triggered`
    (`self.K2_AddActorWorldOffset` (* (+ (* (`self.GetActorForwardVector`) _x) (* (`self.GetActorRightVector`) _y)) 50.0))))

(event `EnhancedInput|/Game/Input/InputActions/Player/IA_Player_ScrollCamera`
  (params (ActionValue :type "Float (double-precision)") (ElapsedSeconds :type "Float (double-precision)") (TriggeredSeconds :type "Float (double-precision)") (InputAction :type "InputAction Object Reference" :default "/Game/Input/InputActions/Player/IA_Player_ScrollCamera.IA_Player_ScrollCamera"))
  (bind _springarm (`self.SpringArm`))
  (bind _returnvalue (- (`SpringArmComponent.TargetArmLength` _springarm) (* ActionValue (`self.CameraScrollSpeed`))))
  (:`Triggered`
    (set `SpringArmComponent.TargetArmLength` (`KismetMathLibrary.FClamp` _returnvalue 500.0 _returnvalue) _springarm)))

(fn `AddMappingContext`
  (bind _asplayer_controller (cast `PlayerController` (`self.GetController`)))
  (`EnhancedInputSubsystemInterface.AddMappingContext` (pcsubsystem `EnhancedInputLocalPlayerSubsystem` _asplayer_controller) "/Game/Input/IMC_PlayerInputs.IMC_PlayerInputs" 0 (struct)))

(fn `AddMovementInputByVector2`
  (params (inVec :type "Vector2D Structure"))
  (bind _capsulecomponent (`self.CapsuleComponent`))
  (bind (_x _y) (`KismetMathLibrary.BreakVector2D` (* inVec (`self.CameraSpeed`))))
  (`PawnMovementComponent.AddInputVector` (`self.CharacterMovement`) (+ (* (`SceneComponent.GetForwardVector` _capsulecomponent) _x) (* (`SceneComponent.GetRightVector` _capsulecomponent) _y)) false))

(fn `GetPlayerID`
  (returns (`Player Id` :type Integer))
  (bind _playerstate (`self.PlayerState`)
    (:`then`
      (return (`PlayerState.PlayerId` _playerstate)))
    (:`else`
      (return 0))))

(fn `LineTraceFromMouseToWorld`
  (params (maxDistance :type "Float (double-precision)" :default 10000.0))
  (returns (Location :type "Vector Structure") (HitActor :type "Actor Object Reference") (Hit :type Boolean) (OutHit :type "HitResult Structure"))
  (bind _returnvalue (`SceneComponent.K2_GetComponentLocation` (`self.Camera`)))
  (bind _thiscontroller (`self.ThisController`)
    (:`then`
      (bind (_outhit _returnvalue_2) (`KismetSystemLibrary.LineTraceSingle` _returnvalue (+ _returnvalue (* (`.WorldDirection` (`PlayerController.DeprojectMousePositionToWorld` _thiscontroller)) maxDistance)) "TraceTypeQuery1"))
      (bind (_bblockinghit _binitialoverlap _time _distance _location _impactpoint _normal _impactnormal _physmat _hitactor) (`GameplayStatics.BreakHitResult` _outhit))
      (return _location _hitactor _returnvalue_2 _outhit))
    (:`else`)))

(fn `MoveByControlInput`
  (params (Delta :type "Float (single-precision)") (MovementInput :type "Vector Structure"))
  (`SceneComponent.K2_SetWorldLocation` (`self.CapsuleComponent`) (+ (* MovementInput Delta) (`self.K2_GetActorLocation`)) false true))

(fn `ProjectScreenLocationToWorld`
  (params (ScreenPos :type "Vector2D Structure") (MaxDistance :type "Float (double-precision)" :default 10000.0))
  (returns (WorldPos :type "Vector Structure"))
  (bind (_x _y) (`KismetMathLibrary.BreakVector2D` ScreenPos))
  (bind _returnvalue (`SceneComponent.K2_GetComponentLocation` (`self.Camera`)))
  (bind _outhit (`KismetSystemLibrary.LineTraceSingle` _returnvalue (+ _returnvalue (* (`.WorldDirection` (`PlayerController.DeprojectScreenPositionToWorld` (`self.ThisController`) _x _y)) MaxDistance)) "TraceTypeQuery1"))
  (return (`.Location` (`GameplayStatics.BreakHitResult` _outhit))))

(fn `RotateCameraByVector2`
  (params (InVec :type "Vector2D Structure"))
  (bind (_x _y) (`KismetMathLibrary.BreakVector2D` InVec))
  (`self.AddControllerYawInput` (* (`self.MouseSensetivity`) (`KismetMathLibrary.SelectFloat` -1.0 1.0 (`self.InvertX`)) _x))
  (`self.AddControllerPitchInput` (* (`self.MouseSensetivity`) (`KismetMathLibrary.SelectFloat` 1.0 -1.0 (`self.InvertY`)) _y)))

(fn `SetInitialValues`
  (`self.ThisController`
    (:`then`
      _)
    (:`else`
      (bind _asbp_player_controller (cast `/Game/Blueprints/Player/BP_PlayerController` (`self.GetController`)))
      (set `self.ThisController` _asbp_player_controller)))
  (`Controller.SetControlRotation` (`self.ThisController`) (`KismetMathLibrary.MakeRotator` 0.0 -45.0 45.0)))

(fn `UserConstructionScript`)