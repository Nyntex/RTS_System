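; Test faction building that highlights on hover with a color based on whether the local player owns it.
; On BeginPlay it compares the first player controller's PlayerState with the PlayerState found as the building's Owner, choosing a custom depth stencil value for own or other.
; Hover and StopHover events write or clear that stencil on the mesh, presumably for an outline post-process.
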(event `self.ReceiveBeginPlay`
  (`self.SetHoverMaterialByRelation` (`Controller.PlayerState` (`GameplayStatics.GetPlayerController` 0))))

(event `/Game/Blueprints/Interfaces/BPI_Selectable.Hover`
  (`PrimitiveComponent.SetCustomDepthStencilValue` (`self.Mesh`) (`self.HoverMaterialDepthNumber`)))

(event `/Game/Blueprints/Interfaces/BPI_Selectable.StopHover`
  (`PrimitiveComponent.SetCustomDepthStencilValue` (`self.Mesh`) 0))

(fn `GetOwningPlayerState`
  (returns (`Player State` :type "PlayerState Object Reference"))
  (bind _asplayer_state (cast `PlayerState` (`self.GetOwner`))
    (:`then`
      (return _asplayer_state))
    (:`CastFailed`
      (return null))))

(fn `SetHoverMaterialByRelation`
  (params (PlayerToCheck :type "PlayerState Object Reference"))
  (bind _player_state (`self.GetOwningPlayerState`))
  (if (and (`KismetSystemLibrary.IsValid` PlayerToCheck) (`KismetSystemLibrary.IsValid` _player_state))
    (if (== (`PlayerState.PlayerId` PlayerToCheck) (`PlayerState.PlayerId` _player_state))
      (set `self.HoverMaterialDepthNumber` 1)
      (else
        (set `self.HoverMaterialDepthNumber` 3)))))

(fn `UserConstructionScript`)