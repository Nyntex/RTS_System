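; Base RTS faction unit that can be hovered, selected and ordered to move to a location.
; Interface events add or remove hover and selection gameplay tags, which toggle custom depth rendering on its sphere.
; On BeginPlay, the stencil value distinguishes units owned by the first local player from all others by comparing player IDs.
; Move orders go through a server RPC to the unit's AI controller via SimpleMoveToLocation.
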(event `self.ReceiveBeginPlay`
  (`self.SetHoverMaterialDepthNumberByRelation` (`Controller.PlayerState` (`GameplayStatics.GetPlayerController` 0))))

(event `/Game/Blueprints/Interfaces/BPI_Selectable.BPI_Hover`
  (`BlueprintGameplayTagLibrary.AddGameplayTag` (`self.GameplayTags`) (struct :`TagName` "RTS.Selection.Hovering"))
  (`self.SetRenderCustomDepthBySelection`))

(event `/Game/Blueprints/Interfaces/BPI_Selectable.BPI_StopHover`
  (`BlueprintGameplayTagLibrary.RemoveGameplayTag` (`self.GameplayTags`) (struct :`TagName` "RTS.Selection.Hovering"))
  (`self.SetRenderCustomDepthBySelection`))

(event `/Game/Blueprints/Interfaces/BPI_Selectable.BPI_Select`
  (`BlueprintGameplayTagLibrary.AddGameplayTag` (`self.GameplayTags`) (struct :`TagName` "RTS.Selection.Selected"))
  (`self.SetRenderCustomDepthBySelection`))

(event `/Game/Blueprints/Interfaces/BPI_Selectable.BPI_Deselect`
  (`BlueprintGameplayTagLibrary.RemoveGameplayTag` (`self.GameplayTags`) (struct :`TagName` "RTS.Selection.Selected"))
  (`self.SetRenderCustomDepthBySelection`))

(event `/Game/Blueprints/Interfaces/BPI_Instructions.BPI_LocationInstruction`
  (params (Location :type "Vector Structure"))
  (`self.Location Instruction (Server)` Location))

(event `Location Instruction (Server)`
  (params (Location :type "Vector Structure"))
  (`AIBlueprintHelperLibrary.SimpleMoveToLocation` (`AIBlueprintHelperLibrary.GetAIController` self) Location)
  (`KismetSystemLibrary.PrintString` "Instructed to move"))

(fn `GetOwningPlayerState`
  (returns (`Player State` :type "PlayerState Object Reference"))
  (`/Engine/EditorBlueprintResources/StandardMacros.IsValid` (`self.OwningPlayerState`)
    (:`Is Valid`
      (return (`self.OwningPlayerState`)))
    (:`Is Not Valid`
      (return null))))

(fn `SetHoverMaterialDepthNumberByRelation`
  (params (PlayerToCheck :type "PlayerState Object Reference"))
  (bind _player_state (`self.GetOwningPlayerState`))
  (bind _sphere (`self.Sphere`))
  (if (and (`KismetSystemLibrary.IsValid` PlayerToCheck) (`KismetSystemLibrary.IsValid` _player_state))
    (if (== (`PlayerState.PlayerId` PlayerToCheck) (`PlayerState.PlayerId` _player_state))
      (`PrimitiveComponent.SetCustomDepthStencilValue` _sphere 1)
      (else
        (`PrimitiveComponent.SetCustomDepthStencilValue` _sphere 3)))
    (else
      (`PrimitiveComponent.SetCustomDepthStencilValue` (`self.Sphere`) 3))))

(fn `SetRenderCustomDepthBySelection`
  (`PrimitiveComponent.SetRenderCustomDepth` (`self.Sphere`) (or (`BlueprintGameplayTagLibrary.HasTag` (`self.GameplayTags`) (struct :`TagName` "RTS.Selection.Hovering")) (`BlueprintGameplayTagLibrary.HasTag` (`self.GameplayTags`) (struct :`TagName` "RTS.Selection.Selected"))))
  (return))

(fn `UserConstructionScript`)