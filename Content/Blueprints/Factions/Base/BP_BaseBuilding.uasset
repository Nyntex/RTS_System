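; Base RTS faction building that handles hover and selection, takes damage and spawns units.
; Gameplay tags toggle a custom-depth outline, with a stencil value set by comparing local and owning players, refreshed on owner replication.
; Damage passes through an armor calculation before reducing health and signaling depletion.
; Selection currently requests a base unit via server RPC, which spawns it from a DataTable row at a traced point beside the building and tracks it until killed.
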(event Custom|TrySpawnUnit%20%28Server%29
  (params (UnitToSpawn :type Data%20Table%20Row%20Handle%20Structure))
  (CallFunction|SpawnUnitBPI UnitToSpawn))

(event EventBeginPlay
  (Outline|SetHoverMaterialDepthNumberbyRelation (Variables|/Script/Engine.Controller|GetPlayerState (Game|GetPlayerController 0))))

(event Collision|EventActorBeginOverlap
  (params (OtherActor :type Actor%20Object%20Reference)))

(event EventTick
  (params (DeltaSeconds :type Float%20%28single-precision%29)))

(event EventBPISelect
  (GameplayTags|AddGameplayTag (Variables|Default|GetGameplayTags) "(TagName=\"RTS.Selection.Selected\")" :!class /Script/GameplayTags.BlueprintGameplayTagLibrary)
  (Outline|SetRenderCustomDepthbySelection)
  (CallFunction|TrySpawnUnitBPI (Utilities|Struct|MakeDataTableRowHandle "/Game/Blueprints/Factions/Base/DT_BaseUnitsTable.DT_BaseUnitsTable" "BaseUnit")))

(event EventBPIStopHover
  (GameplayTags|RemoveGameplayTag (Variables|Default|GetGameplayTags) "(TagName=\"RTS.Selection.Hovering\")" :!class /Script/GameplayTags.BlueprintGameplayTagLibrary)
  (Outline|SetRenderCustomDepthbySelection))

(event EventBPIDeselect
  (GameplayTags|RemoveGameplayTag (Variables|Default|GetGameplayTags) "(TagName=\"RTS.Selection.Selected\")" :!class /Script/GameplayTags.BlueprintGameplayTagLibrary)
  (Outline|SetRenderCustomDepthbySelection))

(event EventBPIHover
  (GameplayTags|AddGameplayTag (Variables|Default|GetGameplayTags) "(TagName=\"RTS.Selection.Hovering\")" :!class /Script/GameplayTags.BlueprintGameplayTagLibrary)
  (Outline|SetRenderCustomDepthbySelection))

(event Game|Damage|EventAnyDamage
  (params (Damage :type Float%20%28single-precision%29) (DamageType :type Damage%20Type%20Object%20Reference) (InstigatedBy :type Controller%20Object%20Reference) (DamageCauser :type Actor%20Object%20Reference))
  (bind _new_damage (Health|RecalculateDamage Damage))
  (bind _depleted (Health|ReduceHealth _new_damage))
  (if _depleted
    (Default|CallHealthDepleted)))

(event EventTrySpawnUnitBPI
  (params (UnitToSpawn :type Data%20Table%20Row%20Handle%20Structure))
  (CallFunction|TrySpawnUnit(Server) UnitToSpawn))

(fn ConstructionScript)

(fn SetHoverMaterialDepthNumberbyRelation
  (params (PlayerToCheck :type Player%20State%20Object%20Reference))
  (bind _player_state (CallFunction|GetOwningPlayerState))
  (bind _mesh (Variables|Default|GetMesh))
  (if (and (Utilities|IsValid PlayerToCheck) (Utilities|IsValid _player_state))
    (if (== (Variables|/Script/Engine.PlayerState|GetPlayerId PlayerToCheck) (Variables|/Script/Engine.PlayerState|GetPlayerId _player_state))
      (Rendering|SetCustomDepthStencilValue _mesh 1)
      (else
        (Rendering|SetCustomDepthStencilValue _mesh 3)))
    (else
      (Rendering|SetCustomDepthStencilValue (Variables|Default|GetMesh) 3))))

(fn GetOwningPlayerState
  (Utilities|IsValid (Variables|Default|GetOwningPlayerState)
    (:Is%20Valid
      (return (Variables|Default|GetOwningPlayerState)))
    (:Is%20Not%20Valid
      (return 0))))

(fn FinishedConstruction
  (return (>= (Variables|Stats|GetConstructionProgress) 1e+02)))

(fn SetRenderCustomDepthbySelection
  (Rendering|SetRenderCustomDepth (Variables|Default|GetMesh) (or (GameplayTags|HasTag (Variables|Default|GetGameplayTags) "(TagName=\"RTS.Selection.Hovering\")") (GameplayTags|HasTag (Variables|Default|GetGameplayTags) "(TagName=\"RTS.Selection.Selected\")")))
  (return))

(fn RecalculateDamage
  (params (Damage :type Float%20%28double-precision%29))
  (return (|(Damage*((ArmorValue+ArmorCalcValue)/ArmorCalcValue)) Damage (Variables|Stats|GetArmorCalculationValue) (Variables|Stats|GetArmor))))

(fn ReduceHealth
  (params (Amount :type Float%20%28double-precision%29))
  (bind _output_get (Variables|Stats|SetCurrentHealth (Math|Float|Clamp(Float) (- (Variables|Stats|GetCurrentHealth) (Math|Float|Clamp(Float) Amount 0.0 (Variables|Stats|GetMaxHealth))) 0.0 (Variables|Stats|GetMaxHealth))))
  (return (<= _output_get 0.0)))

(fn InitialiseDataTableStats
  (bind _returnvalue (Utilities|GetDataTableRow "/Game/Blueprints/DataTables/DT_BuildingData.DT_BuildingData" "BP_BaseBuilding")
    (:then
      (Variables|Stats|SetTotalConstructionProgress (.TotalConstructionProgress (Utilities|Struct|BreakSTR_BuildingData _returnvalue)))
      (Variables|Stats|SetMaxHealth (.MaxHealth (Utilities|Struct|BreakSTR_BuildingData _returnvalue)))
      (Variables|Stats|SetArmor (.Armor (Utilities|Struct|BreakSTR_BuildingData _returnvalue)))
      (Variables|Stats|SetArmorCalculationValue (.ArmorCalculationValue (Utilities|Struct|BreakSTR_BuildingData _returnvalue))))))

(fn OnRepOwningPlayerState
  (Outline|SetHoverMaterialDepthNumberbyRelation (Variables|/Script/Engine.Controller|GetPlayerState (Game|GetPlayerController 0))))

(fn SpawnedUnitKilled
  (params (SelfActor :type BP%20Base%20Unit%20Object%20Reference))
  (Utilities|Array|RemoveItem (Variables|Default|GetSpawnedUnits) SelfActor)
  (EventDispatchers|UnbindEventfromKilled SelfActor (EventDispatchers|CreateEvent :!event SpawnedUnitKilled)))

(fn GetSpawnedUnitsBPI
  (return (Variables|Default|GetSpawnedUnits) true))

(fn SpawnUnitBPI
  (params (UnitToSpawn :type Data%20Table%20Row%20Handle%20Structure))
  (bind (_datatable _rowname) (Utilities|Struct|BreakDataTableRowHandle UnitToSpawn))
  (bind (_origin _boxextent) (Collision|GetActorBounds true true))
  (bind (_x _y _z) (Math|Vector|BreakVector _boxextent))
  (bind _returnvalue (/ _z 2.0))
  (bind _returnvalue_2 (+ _y 1e+02))
  (bind _returnvalue_3 (+ _x 1e+02))
  (bind _returnvalue_4 (+ _origin (Math|Vector|MakeVector _returnvalue_3 _returnvalue_2 _returnvalue)))
  (bind _outhit (Collision|LineTraceByChannel _returnvalue_4 (+ _returnvalue_4 (Math|Vector|MakeVector 0.0 0.0 -1e+03)) "TraceTypeQuery1" false 0 "None"))
  (bind _returnvalue_5 (Utilities|GetDataTableRow _datatable _rowname)
    (:then
      (bind _returnvalue_6 (Game|SpawnActorfromClass (Utilities|Struct|BreakSTR_UnitData _returnvalue_5) (Math|Transform|MakeTransform (.Location (Collision|BreakHitResult _outhit)) "0, 0, 0" "1.000000,1.000000,1.000000") "AdjustIfPossibleButAlwaysSpawn" "MultiplyWithRoot" 0 (Variables|Default|GetOwningPlayerState) 0))
      (Utilities|Array|AddUnique (Variables|Default|GetSpawnedUnits) _returnvalue_6)
      (EventDispatchers|BindEventtoKilled _returnvalue_6 (EventDispatchers|CreateEvent :!event SpawnedUnitKilled))
      (return true))))