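; Scene component that decides whether its owner can be placed, through a CanBePlaced check.
; It scans all child components for primitives tagged as collision checkers and overlap-tests each against WorldStatic objects, ignoring the owner, using the checker's own world transform.
; Placement fails when any tagged primitive overlaps nothing, so each must touch static world; with no valid tagged children it returns true.
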(fn `CanBePlaced`
  (returns (placeable :type Boolean))
  (locals (LocalPlaceable :type Boolean :default false) (LocalComponent :type "SceneComponent Object Reference"))
  (for _array_element (`self.GetChildrenComponents` true)
    (bind _output_get (set `local.LocalComponent` _array_element))
    (if (`self.ComponentHasTag` _output_get (`self.CollisionCheckerTag`))
      (bind _asprimitive_component (cast `PrimitiveComponent` (`local.LocalComponent`))
        (:`then`
          (bind (_outactors _returnvalue) (`KismetSystemLibrary.ComponentOverlapActors` _asprimitive_component (`self.K2_GetComponentToWorld`) (`|MakeArray` "ObjectTypeQuery1" :!type "EObjectTypeQuery Enum") null (`|MakeArray` (`self.GetOwner`))))
          (if (not _returnvalue)
            (`KismetSystemLibrary.PrintString` "No Overlapping Actors")
            (return false)))
        (:`CastFailed`
          (`KismetSystemLibrary.PrintString` "Component is no Primitive Component")))
      (else
        (`KismetSystemLibrary.PrintString` "Component has wrong tag"))))
  (return true))