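; Player character component that handles mouse hover and click selection of world actors.
; Each tick it traces from the camera along the deprojected cursor direction, sending hover messages through BPI_Selectable.
; Enhanced Input clicks select the hovered actor, toggle it off, or clear the previous selection.
; Hold-draw input only records start and cancel mouse positions and draws debug spheres at the traced points.
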(event `self.ReceiveBeginPlay`
  (`self.InitializeVariables`)
  (`self.AddMappingContext`))

(event `self.ReceiveTick`
  (params (DeltaSeconds :type "Float (single-precision)"))
  (bind (_location _hitactor) (`self.LineTraceFromMouseToWorld` 1000000.0))
  (if (!= (`self.CurrentHover`) _hitactor)
    (bind _currenthover (`self.CurrentHover`)
      (:`then`
        (message `/Game/Blueprints/Interfaces/BPI_Selectable.StopHover` _currenthover))
      (:`else`
        _))
    (bind _asbpi_selectable (cast `/Game/Blueprints/Interfaces/BPI_Selectable` _hitactor)
      (:`then`
        (set `self.CurrentHover` _hitactor)
        (`/Game/Blueprints/Interfaces/BPI_Selectable.Hover` _asbpi_selectable))
      (:`CastFailed`
        (set `self.CurrentHover` null)))))

(event `EnhancedInput|/Game/Input/InputActions/PlayerInputs/IA_SelectClick`
  (params (ActionValue :type Boolean) (ElapsedSeconds :type "Float (double-precision)") (TriggeredSeconds :type "Float (double-precision)") (InputAction :type "InputAction Object Reference" :default "/Game/Input/InputActions/PlayerInputs/IA_SelectClick.IA_SelectClick"))
  (:`Triggered`
    (if (== (`self.CurrentSelection`) (`self.CurrentHover`))
      (bind _currentselection (`self.CurrentSelection`)
        (:`then`
          (message `/Game/Blueprints/Interfaces/BPI_Selectable.Deselect` _currentselection)
          (set `self.CurrentSelection` null))
        (:`else`
          (bind _currenthover (`self.CurrentHover` :!label _label)
            (:`then`
              (bind _output_get (set `self.CurrentSelection` _currenthover))
              (message `/Game/Blueprints/Interfaces/BPI_Selectable.Select` _output_get))
            (:`else`
              (set `self.CurrentSelection` null)))))
      (else
        (bind _currentselection_2 (`self.CurrentSelection`)
          (:`then`
            (message `/Game/Blueprints/Interfaces/BPI_Selectable.Deselect` _currentselection_2)
            (goto _label))
          (:`else`
            (goto _label)))))))

(event `EnhancedInput|/Game/Input/InputActions/PlayerInputs/IA_SelectHoldDraw`
  (params (ActionValue :type Boolean) (ElapsedSeconds :type "Float (double-precision)") (TriggeredSeconds :type "Float (double-precision)") (InputAction :type "InputAction Object Reference" :default "/Game/Input/InputActions/PlayerInputs/IA_SelectHoldDraw.IA_SelectHoldDraw"))
  (bind (_locationx _locationy) (`PlayerController.GetMousePosition` (`self.AsOwningPlayerController`)))
  (bind (_locationx_2 _locationy_2) (`PlayerController.GetMousePosition` (`self.AsOwningPlayerController`)))
  (:`Started`
    (set `self.StartMousePosition` (`KismetMathLibrary.MakeVector2D` _locationx_2 _locationy_2))
    (bind _location (`self.LineTraceFromMouseToWorld` 1000000.0))
    (`KismetSystemLibrary.DrawDebugSphere` _location 25.0 12 (struct :`R` 1.0 :`G` 1.0 :`B` 1.0 :`A` 1.0) 1.0))
  (:`Canceled`
    (set `self.EndMousePosition` (`KismetMathLibrary.MakeVector2D` _locationx _locationy))
    (bind _location_2 (`self.LineTraceFromMouseToWorld` 1000000.0))
    (`KismetSystemLibrary.DrawDebugSphere` _location_2 25.0 12 (struct :`R` 1.0 :`G` 1.0 :`B` 1.0 :`A` 1.0) 1.0)))

(fn `AddMappingContext`
  (`EnhancedInputSubsystemInterface.AddMappingContext` (pcsubsystem `EnhancedInputLocalPlayerSubsystem` (`self.AsOwningPlayerController`)) "/Game/Input/IMC_HoveringInputs.IMC_HoveringInputs" 0 (struct)))

(fn `InitializeVariables`
  (bind _asbp_player_character (cast `/Game/Blueprints/Player/BP_PlayerCharacter` (`self.GetOwner`))
    (:`then`
      (bind _asplayer_controller (cast `PlayerController` (`Pawn.GetController` _asbp_player_character))
        (:`then`
          (set `self.AsOwningPlayerController` _asplayer_controller))
        (:`CastFailed`
          (`KismetSystemLibrary.PrintString` "Owning player has no player controller" :!label _label))))
    (:`CastFailed`
      (goto _label)))
  (return))

(fn `LineTraceFromMouseToWorld`
  (params (maxDistance :type "Float (double-precision)" :default 1000000.0))
  (returns (Location :type "Vector Structure") (HitActor :type "Actor Object Reference") (Hit :type Boolean) (OutHit :type "HitResult Structure"))
  (bind _asbp_player_character (cast `/Game/Blueprints/Player/BP_PlayerCharacter` (`self.GetOwner`)))
  (bind _asowningplayercontroller (`self.AsOwningPlayerController`)
    (:`then`
      (bind _returnvalue (`SceneComponent.K2_GetComponentLocation` (`/Game/Blueprints/Player/BP_PlayerCharacter.Camera` _asbp_player_character)))
      (bind _outhit (`KismetSystemLibrary.LineTraceSingle` _returnvalue (+ _returnvalue (* (`.WorldDirection` (`PlayerController.DeprojectMousePositionToWorld` _asowningplayercontroller)) maxDistance)) "TraceTypeQuery1"))
      (bind (_bblockinghit _binitialoverlap _time _distance _location _impactpoint _normal _impactnormal _physmat _hitactor) (`GameplayStatics.BreakHitResult` _outhit))
      (return _location _hitactor _bblockinghit _outhit))
    (:`else`)))