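; Player character component that lets a player issue location instructions to their selected targets.
; On BeginPlay it caches the owning player controller and the sibling mouse hover component, then adds the instructor Enhanced Input mapping context.
; The instruction input traces from the mouse into the world and loops over the hover component's selection.
; Each target gets a server event that forwards the location and instructing player state as a message.
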(event `self.ReceiveBeginPlay`
  (`self.InitializeVariables`)
  (`self.AddMappingContext`))

(event `EnhancedInput|/Game/Input/InputActions/Instructor/IA_Instructor_LocationInstruction`
  (params (ActionValue :type Boolean) (ElapsedSeconds :type "Float (double-precision)") (TriggeredSeconds :type "Float (double-precision)") (InputAction :type "InputAction Object Reference" :default "/Game/Input/InputActions/Instructor/IA_Instructor_LocationInstruction.IA_Instructor_LocationInstruction"))
  (:`Triggered`
    (bind (_hit _outhit _hitactor _returnvalue) (`UtilityFunctions.LineTraceFromMouseToWorld` self))
    (set `self.LatestLocationInstruction` _returnvalue)
    (bind _hovercomponent (`self.HoverComponent`)
      (:`then`
        (for _array_element (`MouseHover_Component.TotalSelection` _hovercomponent)
          (`self.Location Instruction (Server)` _array_element (cast `/Game/Blueprints/Player/BP_PlayerState` (`Controller.PlayerState` (`self.AsOwningPlayerController`)) :!pure true) (`self.LatestLocationInstruction`))))
      (:`else`
        (`KismetSystemLibrary.PrintString` "No Hover Component")))))

(event `Location Instruction (Server)`
  (params (Target :type "Object Object Reference") (InstructingPlayer :type "PlayerState Object Reference") (Location :type "Vector Structure"))
  (message `IInstructions.LocationInstruction` Target InstructingPlayer Location))

(fn `AddMappingContext`
  (bind _asowningplayercontroller (`self.AsOwningPlayerController`))
  (`/Engine/EditorBlueprintResources/StandardMacros.IsValid` _asowningplayercontroller
    (:`Is Valid`
      (`EnhancedInputSubsystemInterface.AddMappingContext` (pcsubsystem `EnhancedInputLocalPlayerSubsystem` _asowningplayercontroller) "/Game/Input/IMC_InstructorInputs.IMC_InstructorInputs" 0 (struct))
      (`KismetSystemLibrary.PrintString` "Added Instructor mapping context"))
    (:`Is Not Valid`
      (`KismetSystemLibrary.PrintString` "Owning Player Controller is invalid"))))

(fn `InitializeVariables`
  (`|ExecutionSequence`
    (:`then_0`
      ;[1 1 1] Setup Owning Player Controller
      (bind _asbp_player_character (cast `/Game/Blueprints/Player/BP_PlayerCharacter` (`self.GetOwner`))
        (:`then`
          (bind _asplayer_controller (cast `PlayerController` (`Pawn.GetController` _asbp_player_character))
            (:`then`
              (set `self.AsOwningPlayerController` _asplayer_controller))
            (:`CastFailed`
              (`KismetSystemLibrary.PrintString` "Owning player has no player controller" :!label _label))))
        (:`CastFailed`
          (goto _label))))
    (:`then_1`
      ;[1 1 1] Setup Mouse Hover component
      (set `self.HoverComponent` (`Actor.GetComponentByClass` (`self.GetOwner`) "/Game/Blueprints/Components/BPC_MouseHover.BPC_MouseHover_C")))
    (:`then_2`
      (return))))