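; Player camera pawn with RTS-style controls for moving, looking, hovering over selectables and placing test buildings.
; Enhanced Input feeds camera rotation and movement, which Tick applies by teleporting the root.
; Cursor traces drive BPI_Selectable hover and key 2's RPC spawning of an owner-tagged BP_TestBuilding.
; Drag selection only draws debug shapes; click selection and the movement RPC are unfinished stubs.
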(event Custom|RPC_MoveActor
  (params (Delta :type Float%20%28single-precision%29) (MovementInput :type Vector)))

(event Custom|RPC_Server_Spawn
  (params (PlayerOwner :type Integer) (Spawn%20Transform%20Location :type Vector) (Owner :type Actor%20Object%20Reference))
  (CallFunction|RPCSpawn PlayerOwner Spawn%20Transform%20Location Owner))

(event Custom|RPC_Spawn
  (params (PlayerOwner :type Integer) (Spawn%20Transform%20Location :type Vector) (Owner :type Actor%20Object%20Reference))
  (bind _returnvalue (Game|SpawnActorfromClass "/Game/Factions/Test/BP_TestBuilding.BP_TestBuilding_C" (Math|Transform|MakeTransform Spawn%20Transform%20Location "0, 0, 0" "1.000000,1.000000,1.000000") "Undefined" "MultiplyWithRoot" Owner 0))
  (Variables|/Game/Factions/Test/BP_TestBuilding.BP_TestBuilding_C|SetPlayerOwner _returnvalue PlayerOwner))

(event Custom|RPC_Server_MoveActor
  (params (Delta :type Float%20%28single-precision%29) (MovementInput :type Vector))
  (CallFunction|RPCMoveActor Delta MovementInput))

(event Input|EnhancedActionEvents|EnhancedInputActionIA_MoveCamera
  (params (ActionValue :type Vector%202D%20Structure) (ElapsedSeconds :type Float%20%28double-precision%29) (TriggeredSeconds :type Float%20%28double-precision%29) (InputAction :type Input%20Action%20Object%20Reference :default "/Game/Input/InputActions/PlayerInputs/IA_MoveCamera.IA_MoveCamera"))
  (CallFunction|RotateCamerabyVector2 ActionValue))

(event Input|EnhancedActionEvents|EnhancedInputActionIA_Move
  (params (ActionValue :type Vector%202D%20Structure) (ElapsedSeconds :type Float%20%28double-precision%29) (TriggeredSeconds :type Float%20%28double-precision%29) (InputAction :type Input%20Action%20Object%20Reference :default "/Game/Input/InputActions/PlayerInputs/IA_Move.IA_Move"))
  (CallFunction|AddMovementInputbyVector2 ActionValue))

(event Input|EnhancedActionEvents|EnhancedInputActionIA_SelectHoldDraw
  (params (ActionValue :type Boolean) (ElapsedSeconds :type Float%20%28double-precision%29) (TriggeredSeconds :type Float%20%28double-precision%29) (InputAction :type Input%20Action%20Object%20Reference :default "/Game/Input/InputActions/PlayerInputs/IA_SelectHoldDraw.IA_SelectHoldDraw"))
  (bind _thiscontroller (Variables|Components|GetThisController))
  (bind _thiscontroller_2 (Variables|Components|GetThisController))
  (bind (_locationx _locationy) (Game|Player|GetMousePosition _thiscontroller))
  (bind (_locationx_2 _locationy_2) (Game|Player|GetMousePosition _thiscontroller_2))
  (:Started
    (Variables|Default|SetStartMousePosition (Math|Vector2D|MakeVector2D _locationx_2 _locationy_2))
    (bind _location (CallFunction|LineTracefromMousetoWorld 1e+04))
    (Rendering|Debug|DrawDebugSphere _location 25.0 12 "(R=1.000000,G=1.000000,B=1.000000,A=1.000000)" 1.0))
  (:Canceled
    (Variables|Default|SetEndMousePosition (Math|Vector2D|MakeVector2D _locationx _locationy))
    (bind _location_2 (CallFunction|LineTracefromMousetoWorld 1e+04))
    (Rendering|Debug|DrawDebugSphere _location_2 5.0 12 "(R=0.000000,G=0.000000,B=1.000000,A=1.000000)" 1.0)
    (Rendering|Debug|DrawDebugSphere (CallFunction|ProjectScreenLocationtoWorld (Variables|Default|GetStartMousePosition) 1e+04) 5.0 12 "(R=0.000000,G=0.000000,B=1.000000,A=1.000000)" 1.0 5.0)
    (Rendering|Debug|DrawDebugSphere (|(((VecA-VecB)*0.500000)+VecB) (CallFunction|ProjectScreenLocationtoWorld (Variables|Default|GetStartMousePosition) 1e+04) (CallFunction|ProjectScreenLocationtoWorld (Variables|Default|GetEndMousePosition) 1e+04)) 5.0 12 "(R=1.000000,G=0.000000,B=0.000000,A=1.000000)" 1.0 5.0)
    (Rendering|Debug|DrawDebugBox :Center (|(((VecA-VecB)*0.500000)+VecB) (CallFunction|ProjectScreenLocationtoWorld (Variables|Default|GetStartMousePosition) 1e+04) (CallFunction|ProjectScreenLocationtoWorld (Variables|Default|GetEndMousePosition) 1e+04)) :Extent (Math|Vector|MakeVector (.X (Math|Vector|BreakVector (- (CallFunction|ProjectScreenLocationtoWorld (Variables|Default|GetStartMousePosition) 1e+04) (CallFunction|ProjectScreenLocationtoWorld (Variables|Default|GetEndMousePosition) 1e+04)))) (.Y (Math|Vector|BreakVector (- (CallFunction|ProjectScreenLocationtoWorld (Variables|Default|GetStartMousePosition) 1e+04) (CallFunction|ProjectScreenLocationtoWorld (Variables|Default|GetEndMousePosition) 1e+04)))) 5.0) :Rotation (Math|Rotator|MakeRotator 0.0 0.0 (.Yaw (Math|Rotator|BreakRotator (Transformation|GetWorldRotation (Variables|Default|GetCube))))) :Duration 1.0 :Thickness 3.0)))

(event Input|EnhancedActionEvents|EnhancedInputActionIA_SelectClick
  (params (ActionValue :type Boolean) (ElapsedSeconds :type Float%20%28double-precision%29) (TriggeredSeconds :type Float%20%28double-precision%29) (InputAction :type Input%20Action%20Object%20Reference :default "/Game/Input/InputActions/PlayerInputs/IA_SelectClick.IA_SelectClick")))

(event EventBeginPlay
  (CallFunction|AddMappingContext)
  (CallFunction|SetInitialValues)
  (Actor|SetOwner (Variables|Components|GetThisController)))

(event Collision|EventActorBeginOverlap
  (params (OtherActor :type Actor%20Object%20Reference)))

(event EventTick
  (params (DeltaSeconds :type Float%20%28single-precision%29))
  (bind _returnvalue (Class|Pawn|ConsumeMovementInputVector))
  (CallFunction|MovebyControlInput DeltaSeconds _returnvalue)
  (bind _hitactor (CallFunction|LineTracefromMousetoWorld 1e+04))
  (if (!= _hitactor (Variables|Default|GetCurrentHover))
    (bind _currenthover (Variables|Default|GetCurrentHover)
      (:then
        (Class|BPISelectable|StopHover(Message) _currenthover))
      (:else
        _))
    (bind _asbpi_selectable (Utilities|Casting|CastToBPI_Selectable _hitactor)
      (:then
        (Variables|Default|SetCurrentHover _hitactor)
        (bind _playerstate (Variables|GetPlayerState)
          (:then
            (Default|Hover _asbpi_selectable (Variables|/Script/Engine.PlayerState|GetPlayerId _playerstate))
            (bind _asbp_test_building (Utilities|Casting|CastToBP_TestBuilding _hitactor))
            (Default|RPCServerHover _asbp_test_building (Variables|/Script/Engine.PlayerState|GetPlayerId _playerstate)))
          (:else)))
      (:CastFailed
        (Variables|Default|SetCurrentHover 0)))))

(event Input|KeyboardEvents|2
  (params (Key :type Key%20Structure :default "None"))
  (:Pressed
    (bind _playerstate (Variables|GetPlayerState)
      (:then
        (bind _location (CallFunction|LineTracefromMousetoWorld 1e+04))
        (CallFunction|RPCServerSpawn (Variables|/Script/Engine.PlayerState|GetPlayerId _playerstate) _location (Variables|Components|GetThisController)))
      (:else))))

(fn ConstructionScript)

(fn RotateCamerabyVector2
  (params (InVec :type Vector%202D%20Structure))
  (bind (_x _y) (Math|Vector2D|BreakVector2D InVec))
  (Pawn|Input|AddControllerYawInput (|((Sensetivity*(Invertion*negative))*ActionValue) (Variables|Camera|GetMouseSensetivity) (Math|Float|SelectFloat 1.0 -1.0 (Variables|Camera|GetInvertX)) -1.0 _x))
  (Pawn|Input|AddControllerPitchInput (|((Sensetivity*(Invertion*negative))*ActionValue) (Variables|Camera|GetMouseSensetivity) (Math|Float|SelectFloat -1.0 1.0 (Variables|Camera|GetInvertY)) -1.0 _y)))

(fn AddMappingContext
  (bind _asplayer_controller (Utilities|Casting|CastToPlayerController (Pawn|GetController)))
  (Input|AddMappingContext (PlayerController|LocalPlayerSubsystems|GetEnhancedInputLocalPlayerSubsystem _asplayer_controller) "/Game/Input/IMC_PlayerInputs.IMC_PlayerInputs" 0 "(bIgnoreAllPressedKeysUntilRelease=True,bForceImmediately=False,bNotifyUserSettings=False)"))

(fn SetInitialValues
  (Variables|Components|GetThisController
    (:then
      _)
    (:else
      (bind _asbp_player_controller (Utilities|Casting|CastToBP_PlayerController (Pawn|GetController)))
      (Variables|Components|SetThisController _asbp_player_controller)))
  (Pawn|SetControlRotation (Variables|Components|GetThisController) (Math|Rotator|MakeRotator 0.0 -45.0 45.0)))

(fn AddMovementInputbyVector2
  (params (inVec :type Vector%202D%20Structure))
  (bind _defaultsceneroot (Variables|Default|GetDefaultSceneRoot))
  (bind _cameraspeed (Variables|Camera|GetCameraSpeed))
  (bind _returnvalue (* inVec _cameraspeed))
  (bind (_x _y) (Math|Vector2D|BreakVector2D _returnvalue))
  (Pawn|Input|AddMovementInput (+ (* (Math|Vector|GetForwardVector _defaultsceneroot) _x) (* (Math|Vector|GetRightVector _defaultsceneroot) _y)) 1.0 false))

(fn LineTracefromMousetoWorld
  (params (maxDistance :type Float%20%28double-precision%29))
  (bind _camera (Variables|Default|GetCamera))
  (bind _returnvalue (Transformation|GetWorldLocation _camera))
  (bind _thiscontroller (Variables|Components|GetThisController)
    (:then
      (bind (_outhit _returnvalue_2) (Collision|LineTraceByChannel _returnvalue (+ _returnvalue (* (.WorldDirection (Game|Player|ConvertMouseLocationToWorldSpace _thiscontroller)) maxDistance)) "TraceTypeQuery1" false 0 "None"))
      (return (.Location (Collision|BreakHitResult _outhit)) (.HitActor (Collision|BreakHitResult _outhit)) _returnvalue_2 _outhit))
    (:else)))

(fn ProjectScreenLocationtoWorld
  (params (ScreenPos :type Vector%202D%20Structure) (MaxDistance :type Float%20%28double-precision%29))
  (bind (_x _y) (Math|Vector2D|BreakVector2D ScreenPos))
  (bind _camera (Variables|Default|GetCamera))
  (bind _returnvalue (Transformation|GetWorldLocation _camera))
  (bind _outhit (Collision|LineTraceByChannel _returnvalue (+ _returnvalue (* (.WorldDirection (Class|PlayerController|DeprojectScreenPositiontoWorld (Variables|Components|GetThisController) _x _y)) MaxDistance)) "TraceTypeQuery1" false 0 "None"))
  (return (.Location (Collision|BreakHitResult _outhit))))

(fn MovebyControlInput
  (params (Delta :type Float%20%28single-precision%29) (MovementInput :type Vector))
  (Transformation|SetWorldLocation (Variables|Default|GetDefaultSceneRoot) (+ (* MovementInput Delta) (Transformation|GetActorLocation)) false true))